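; Player controller for the Castle part of RunAndDodge that toggles a pause menu with the Z key.
; Opening creates the WBP_PauseMenu widget once, passes itself to it, then reuses it on later opens, showing the cursor, switching to game-and-UI input and pausing the game.
; Closing removes the widget and restores game-only input, hidden cursor and unpaused play.
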(event `Key|Z` :paused true
  (params (Key :type "Key Structure"))
  (:`Pressed`
    (if (`self.bIsPauseMenuOn`)
      (`self.DeletePauseMenuWidget`)
      (else
        (`self.CreatePauseMenuWidget`)))))

(fn `CreatePauseMenuWidget`
  (bind _pausemenuwidget (`self.PauseMenuWidget`)
    (:`then`
      (`UserWidget.AddToViewport` _pausemenuwidget 0)
      (set `self.bShowMouseCursor` true)
      (`WidgetBlueprintLibrary.SetInputMode_GameAndUIEx` self null "DoNotLock" false)
      (`GameplayStatics.SetGamePaused` true)
      (set `self.bIsPauseMenuOn` true))
    (:`else`
      (bind _returnvalue (`|CreateWidget` "/Game/RunAndDodge/UI/DuringTheGame/WBP_PauseMenu.WBP_PauseMenu_C" self))
      (bind _output_get (set `self.PauseMenuWidget` _returnvalue))
      (set `/Game/RunAndDodge/UI/DuringTheGame/WBP_PauseMenu.playerController` self _output_get)
      (`UserWidget.AddToViewport` _output_get 0)
      (set `self.bShowMouseCursor` true)
      (`WidgetBlueprintLibrary.SetInputMode_GameAndUIEx` self null "DoNotLock" false)
      (`GameplayStatics.SetGamePaused` true)
      (set `self.bIsPauseMenuOn` true))))

(fn `DeletePauseMenuWidget`
  (`Widget.RemoveFromParent` (`self.PauseMenuWidget`))
  (set `self.bShowMouseCursor` false)
  (`WidgetBlueprintLibrary.SetInputMode_GameOnly` self)
  (`GameplayStatics.SetGamePaused` false)
  (set `self.bIsPauseMenuOn` false))

(fn `UserConstructionScript`)